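; GI_Main, by its name the main game instance, exposes two events that adjust the timer and score held on BP_Gamemode.
; DecreaseTime subtracts a fixed amount from the game mode's Time, and AddScore increments its Score by one.
; Each event casts the current game mode to BP_Gamemode and does nothing if the cast fails.
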(event `DecreaseTime`
  ;[1 1 1] Decrease the time passed
  (bind _asbp_gamemode (cast `/Game/Blueprints/BP_Gamemode` (`GameplayStatics.GetGameMode`)))
  (set `/Game/Blueprints/BP_Gamemode.Time` (- (`/Game/Blueprints/BP_Gamemode.Time` _asbp_gamemode) 10.0) _asbp_gamemode))

(event `AddScore`
  ;[1 1 1] Add a point
  (bind _asbp_gamemode (cast `/Game/Blueprints/BP_Gamemode` (`GameplayStatics.GetGameMode`)))
  (set `/Game/Blueprints/BP_Gamemode.Score` (+ (`/Game/Blueprints/BP_Gamemode.Score` _asbp_gamemode) 1) _asbp_gamemode))